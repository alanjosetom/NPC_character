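; Sword-and-shield enemy NPC character with a health bar widget, driven by an AI controller and a damage system component.
; Hits freeze it, then switch the AI to attack the causer; death ragdolls it and stops AI logic.
; Montage-driven attacks sphere-trace on notify, while blocking uses a state enum and reaction montage, both signalling completion through dispatchers.
; Interface functions forward health and damage to the component; Attack and SetMoveSpeed are unwired.
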(event `self.ReceiveBeginPlay`
  (bind _bpc_damagesystem (`self.BPC_DamageSystem`))
  (bind _asai_controller (cast `/Game/AI/AI_Controller` (`AIBlueprintHelperLibrary.GetAIController` self)))
  (set `self.AI_Enemy` _asai_controller)
  (bind _returnvalue (`|CreateWidget` "/Game/AI/DamageSystem/W_HealthBar.W_HealthBar_C" null self))
  (`WidgetComponent.SetWidget` (`self.HealthBar`) _returnvalue)
  (add `/Game/AI/DamageSystem/BPC_DamageSystem.OnDeath` _bpc_damagesystem (`|CreateDelegate` :!event `Die`))
  (add `/Game/AI/DamageSystem/BPC_DamageSystem.OnDamageResponse` _bpc_damagesystem (`|CreateDelegate` :!event `HitResponse`)))

(event `Die`
  (bind _mesh (`self.Mesh`))
  (`PrimitiveComponent.SetSimulatePhysics` _mesh true)
  (`PrimitiveComponent.SetCollisionEnabled` _mesh "QueryAndPhysics")
  (`BrainComponent.StopLogic` (`AIController.BrainComponent` (`self.AI_Enemy`)) "")
  (`/Game/AI/AI_Controller.SetStatedead` (`self.AI_Enemy`)))

(event `HitResponse`
  (params (DamageResponse :type "/Game/AI/DamageSystem/E_DamageResponse Enum" :default "NewEnumerator0") (DamageCauser :type "Actor Object Reference"))
  (`MovementComponent.StopMovementImmediately` (`self.CharacterMovement`))
  (`/Game/AI/AI_Controller.SetStateFrozen` (`self.AI_Enemy`))
  (`|PlayMontage` (`self.Mesh`) "/Game/Characters/Mannequins/Animations/Manny/sword-shield-hit_Montage.sword-shield-hit_Montage"
    (:`OnCompleted`
      _)
    (:`OnInterrupted`
      _))
  (`/Game/AI/AI_Controller.SetStateAttacking` (`self.AI_Enemy`) DamageCauser true))

(event `AttackPlayer`
  (bind _returnvalue (`self.K2_GetActorLocation`))
  (bind _notifyname (`|PlayMontage` (`self.Mesh`) "/Game/Characters/Mannequins/Animations/Manny/sword-slash_Montage.sword-slash_Montage")
    (:`then`
      (set `/Game/AI/DamageSystem/BPC_DamageSystem.IsInterruptible` false (`self.BPC_DamageSystem`)))
    (:`OnCompleted`
      (`self.OnAttackEnd` :!label _label)
      (set `/Game/AI/DamageSystem/BPC_DamageSystem.IsInterruptible` true (`self.BPC_DamageSystem`)))
    (:`OnInterrupted`
      (goto _label))
    (:`OnNotifyBegin`
      (switch `name` _notifyname
        (:`Trace`
          (bind (_outhit _returnvalue_2) (`KismetSystemLibrary.SphereTraceSingleForObjects` :`Start` _returnvalue :`End` (+ _returnvalue (* (`self.GetActorForwardVector`) 200.0)) :`Radius` 20.0 :`ObjectTypes` (`|MakeArray` "ObjectTypeQuery3" :!type "EObjectTypeQuery Enum") :`DrawDebugType` "ForDuration"))
          (if _returnvalue_2
            (message `/Game/AI/DamageSystem/BPI_Damagable.TakeDamage` (`.HitActor` (`GameplayStatics.BreakHitResult` _outhit)) (make `/Game/AI/DamageSystem/S_DamageInfo` 25.0 "NewEnumerator1") self)))))))

(event `self.ReceiveHit`
  (params (MyComp :type "PrimitiveComponent Object Reference") (Other :type "Actor Object Reference") (OtherComp :type "PrimitiveComponent Object Reference") (bSelfMoved :type Boolean) (HitLocation :type "Vector Structure") (HitNormal :type "Vector Structure") (NormalImpulse :type "Vector Structure") (Hit :type "HitResult Structure (by ref)"))
  (`AISense_Touch.ReportTouchEvent` self Other HitLocation))

(event `StartBlock`
  (`MovementComponent.StopMovementImmediately` (`self.CharacterMovement`))
  (set `/Game/AI/DamageSystem/BPC_DamageSystem.IsBlocking` true (`self.BPC_DamageSystem`))
  (set `self.BlockingState` "NewEnumerator1")
  (`|PlayMontage` (`self.Mesh`) "/Game/Characters/Mannequins/Animations/Manny/sword-block_Montage.sword-block_Montage"
    (:`OnCompleted`
      (`self.EndBlock` :!label _label_2))
    (:`OnInterrupted`
      (if (`|EnumInequality` (`self.BlockingState`) "NewEnumerator2")
        (goto _label_2)))))

(event `self.BPC_DamageSystem.OnBlocked`
  (params (CanBeParried :type Boolean))
  (set `self.BlockingState` "NewEnumerator2")
  (`|PlayMontage` (`self.Mesh`) "/Game/Characters/Mannequins/Animations/Manny/sword-block-react_Montage.sword-block-react_Montage"
    (:`OnCompleted`
      _)
    (:`OnInterrupted`
      _))
  (`self.EndBlock`))

(event `EndBlock`
  (set `self.BlockingState` "NewEnumerator0")
  (set `/Game/AI/DamageSystem/BPC_DamageSystem.IsBlocking` false (`self.BPC_DamageSystem`))
  (`self.OnBlockEnded`))

(fn `Attack`
  (returns (`Animation Durartion` :type "Float (double-precision)")))

(fn `GetCurrentHealth`
  (returns (Health :type "Float (double-precision)"))
  (return (`/Game/AI/DamageSystem/BPC_DamageSystem.Health` (`self.BPC_DamageSystem`))))

(fn `GetIdleRange`
  (returns (AttackRadius :type "Float (double-precision)") (DefendRadius :type "Float (double-precision)"))
  (return 150.0 350.0))

(fn `GetMaxHealth`
  (returns (MaxHealth :type "Float (double-precision)"))
  (return (`/Game/AI/DamageSystem/BPC_DamageSystem.MaxHealth` (`self.BPC_DamageSystem`))))

(fn `GetPatrolPath`
  (returns (PatrolPath :type "/Game/AI/BP_PatrolRoute Object Reference"))
  (return (`self.PatrolRoute`)))

(fn `Heal`
  (params (Amount :type "Float (double-precision)"))
  (returns (NewHealth :type "Float (double-precision)"))
  (bind _newhealth (`/Game/AI/DamageSystem/BPC_DamageSystem.Heal` (`self.BPC_DamageSystem`) Amount))
  (return _newhealth))

(fn `IsAttacking`
  (returns (Attacking :type Boolean))
  (return false))

(fn `IsDead`
  (returns (Dead :type Boolean))
  (return (`/Game/AI/DamageSystem/BPC_DamageSystem.IsDead` (`self.BPC_DamageSystem`))))

(fn `SetMoveSpeed`
  (params (Speed :type "/Game/AI/Enum/MoveSpeed Enum" :default "NewEnumerator0"))
  (returns (SpeedValue :type "Float (double-precision)"))
  (return 0.0))

(fn `TakeDamage`
  (params (DamageInfo :type "/Game/AI/DamageSystem/S_DamageInfo Structure") (`Damage Causer` :type "Actor Object Reference"))
  (returns (WasDamaged :type Boolean))
  (bind _wasdamaged (`/Game/AI/DamageSystem/BPC_DamageSystem.TakeDamage` (`self.BPC_DamageSystem`) DamageInfo `Damage Causer`))
  (return _wasdamaged))

(fn `UserConstructionScript`
  (bind _bpc_damagesystem (`self.BPC_DamageSystem`))
  (set `/Game/AI/DamageSystem/BPC_DamageSystem.MaxHealth` 100.0 _bpc_damagesystem)
  (set `/Game/AI/DamageSystem/BPC_DamageSystem.Health` 100.0 _bpc_damagesystem))