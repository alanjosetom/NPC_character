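; BPC_Attacks is an attack component that casts a homing-capable dark energy projectile for its owning actor.
; MagicSpell spawns BP_Projectile_DarkEnergy with a target, ignores the owner in its collision and binds its impact delegate.
; On impact, it sends the spell's damage info through a TakeDamage message, reports an AI damage event and calls OnAttackEnded.
; Fire is an empty event, with its line-trace damage logic left disconnected.
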(event `MagicSpell`
  (params (SpawnTransform :type "Transform Structure") (Target :type "Actor Object Reference") (DamageInfo :type "/Game/AI/DamageSystem/S_DamageInfo Structure"))
  (bind _returnvalue (`|SpawnActorFromClass` "/Game/Projectiles/BP_Projectile_DarkEnergy.BP_Projectile_DarkEnergy_C" SpawnTransform "Undefined" "MultiplyWithRoot" (`self.GetOwner`) 1000.0 0.0 Target false null))
  (add `/Game/Projectiles/BP_Projectile_Base.OnProjectileImpact` _returnvalue (delegate `OnProjectHit`))
  (`PrimitiveComponent.IgnoreActorWhenMoving` (`/Game/Projectiles/BP_Projectile_Base.BoxCollision` _returnvalue) (`self.GetOwner`) true))

(event `OnProjectHit`
  (params (OtherActor :type "Actor Object Reference") (Hit :type "HitResult Structure"))
  (bind _returnvalue (`self.GetOwner`))
  (message `/Game/AI/DamageSystem/BPI_Damagable.TakeDamage` OtherActor (stale `MagicSpell` DamageInfo) _returnvalue)
  (`AISense_Damage.ReportDamageEvent` OtherActor _returnvalue (`.Amount_2_64864A0D4320D27C3EA14D8019B5EC9D` (break `/Game/AI/DamageSystem/S_DamageInfo` (stale `MagicSpell` DamageInfo))) (`Actor.K2_GetActorLocation` (`self.GetOwner`)))
  (`self.OnAttackEnded`))

(event `Fire`
  (params (TraceStart :type "Vector Structure") (TraceEnd :type "Vector Structure") (DamageInfo :type "/Game/AI/DamageSystem/S_DamageInfo Structure"))
  ;[1 1 1] if delete
)